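; BP_NPC_Knight_Haveron is a knight NPC child Blueprint for the character named Haveron.
; On BeginPlay it sets its name, gathers NPC_POI actors tagged with that name as its patrol points, then runs the parent BeginPlay.
; When interacted with, it notifies every quest in the player's quest log that it was interacted with.
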(event EventBeginPlay
  (bind _output_get (Variables|Default|SetName "Haveron"))
  (bind _outactors (Actor|GetAllActorsOfClasswithTag "/Game/AI/POIS/NPC_POI.NPC_POI_C" (Utilities|String|StringToName _output_get)))
  (Variables|Default|SetPatrol%20Points _outactors)
  (|CallParentFunction))

(event EventInteract
  (bind _asplayer_character (Utilities|Casting|CastToPlayerCharacter (Game|GetPlayerCharacter 0)))
  (for _array_element (Variables|/Game/QuestSystem/Blueprints/BP_QuestLog.BP_QuestLog_C|GetQuests (Variables|/Game/ThirdPersonCharacter/PlayerCharacter.PlayerCharacter_C|GetBP_QuestLog _asplayer_character))
    (Default|CallInteracted _array_element self)))

(event EventTick
  (params (DeltaSeconds :type Float%20%28single-precision%29)))

(event Collision|EventActorBeginOverlap
  (params (OtherActor :type Actor%20Object%20Reference)))

(fn ConstructionScript
  (|CallParentFunction))