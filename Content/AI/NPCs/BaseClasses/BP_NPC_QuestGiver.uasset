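; Base quest-giver NPC that reports player interactions to each active quest in the player's quest log.
; On BeginPlay it starts wandering between random ShopKeep-tagged points of interest, pausing after each successful move.
; Hardcoded logic for the NewBeginnings quest removes Jolleen at BeginPlay if it is completed.
; ActorDisappear checks for that completed quest, then spawns sparkles and drives a dynamic material's opacity by timeline before destroying the actor.
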(event Custom|Walk%20Around
  (bind _poi (Variables|Default|GetPOI))
  (bind _output_get (Variables|Default|SetTarget%20POI (Utilities|Array|Get(acopy) _poi (Math|Random|RandomIntegerinRange 0 (Utilities|Array|Length _poi)))))
  (AI|AIMoveTo self "0, 0, 0" _output_get 5.0 false
    (:OnSuccess
      (Utilities|FlowControl|Delay 3.0)
      (CallFunction|WalkAround))))

(event Custom|Actor%20Disappear
  (params (Player :type Player%20Character%20Object%20Reference))
  (for _array_element (Variables|/Game/QuestSystem/Blueprints/BP_QuestLog.BP_QuestLog_C|GetCompleted%20Quests (Variables|/Game/ThirdPersonCharacter/PlayerCharacter.PlayerCharacter_C|GetBP_QuestLog Player))
    (if (Utilities|Enum|Equal(Enum) (Utilities|GetDisplayName _array_element) "BPQ_NewBeginnings")
      (Utilities|FlowControl|Delay 0.2)
      (Effects|SpawnEmitteratLocation "/Game/FX/Sparkles/P_Sparkles_Jolleen.P_Sparkles_Jolleen" (+ (Transformation|GetActorLocation) "0, 0,30.000000"))
      ;[1 1 1] Change to fade out
      (CallFunction|FadeOutMaterial))))

(event Custom|FadeOutMaterial
  (Rendering|Material|SetMaterial (Variables|Character|GetMesh) 0 (Variables|Default|GetMaterialToChange))
  (bind _returnvalue (Rendering|Material|CreateDynamicMaterialInstance (Variables|Default|GetMaterialToChange) "DynamicMaterial_Jolleen" :!class /Script/Engine.KismetMaterialLibrary))
  (bind _output_get (Variables|Default|SetNewDynamicMat _returnvalue))
  (Rendering|Material|SetMaterial (Variables|Character|GetMesh) 0 _output_get)
  (bind _percentage (Timeline|Timeline_0 Play)
    (:Update
      (Rendering|Material|SetScalarParameterValue (Variables|Default|GetNewDynamicMat) "Opacity" _percentage :!class /Script/Engine.MaterialInstanceDynamic))
    (:Finished
      (Actor|DestroyActor))))

(event EventBeginPlay
  (bind _asplayer_character (Utilities|Casting|CastToPlayerCharacter (Game|GetPlayerCharacter 0)))
  (for _array_element (Variables|/Game/QuestSystem/Blueprints/BP_QuestLog.BP_QuestLog_C|GetCompleted%20Quests (Variables|/Game/ThirdPersonCharacter/PlayerCharacter.PlayerCharacter_C|GetBP_QuestLog _asplayer_character))
    (if (and (Utilities|Enum|Equal(Enum) (Utilities|GetDisplayName _array_element) "BPQ_NewBeginnings") (Variables|/Game/QuestSystem/Quests/BP_Quest.BP_Quest_C|GetisCompleted? _array_element))
      (if (Utilities|Enum|Equal(Enum) (Variables|Default|GetSelfName) "Jolleen")
        (Actor|DestroyActor))))
  (bind _outactors (Actor|GetAllActorsOfClasswithTag "/Game/AI/POIS/NPC_POI.NPC_POI_C" "ShopKeep"))
  (Variables|Default|SetPOI _outactors)
  (CallFunction|WalkAround)
  (|CallParentFunction))

(event EventInteract
  (bind _asplayer_character (Utilities|Casting|CastToPlayerCharacter (Game|GetPlayerCharacter 0)))
  (for _array_element (Variables|/Game/QuestSystem/Blueprints/BP_QuestLog.BP_QuestLog_C|GetQuests (Variables|/Game/ThirdPersonCharacter/PlayerCharacter.PlayerCharacter_C|GetBP_QuestLog _asplayer_character))
    (Default|CallInteracted _array_element self)))

(event EventTick
  (params (DeltaSeconds :type Float%20%28single-precision%29))
  (|CallParentFunction DeltaSeconds) ; This node is disabled and will not be called.\nDrag off pins to build functionality.
)

(event Collision|EventActorBeginOverlap
  (params (OtherActor :type Actor%20Object%20Reference))
  (|CallParentFunction OtherActor) ; This node is disabled and will not be called.\nDrag off pins to build functionality.
)

(fn ConstructionScript
  (|CallParentFunction))