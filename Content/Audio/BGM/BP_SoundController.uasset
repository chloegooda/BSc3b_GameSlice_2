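; BP_SoundController plays background music and swaps the track to suit the game level.
; On BeginPlay it starts its AudioComponent and then flags it as a UI sound.
; UpdateBGM stops the component and sets the sound by level, with Farm and Grasslands sharing the farm loop and Market Persistent using the market track.
; UpdateBGM makes no Play call after changing the sound.
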(event EventBeginPlay
  (Audio|Components|Audio|Play (Variables|Components|GetAudioComponent) 0.0)
  (Class|AudioComponent|SetUISound (Variables|Components|GetAudioComponent) true))

(event EventTick
  (params (DeltaSeconds :type Float%20%28single-precision%29)))

(fn ConstructionScript)

(fn UpdateBGM
  (params (Level :type ListOfLevels%20Enum :default "NewEnumerator0"))
  (bind _audiocomponent (Variables|Components|GetAudioComponent))
  (Audio|Components|Audio|Stop (Variables|Components|GetAudioComponent))
  (switch Utilities|FlowControl|Switch|SwitchonListOfLevels Level
    (:NewEnumerator6
      (Audio|Components|Audio|SetSound _audiocomponent "/Game/Audio/BGM/SC_BGM_FarmLoop.SC_BGM_FarmLoop"))
    (:NewEnumerator7
      (Audio|Components|Audio|SetSound _audiocomponent "/Game/Audio/BGM/SC_BGM_FarmLoop.SC_BGM_FarmLoop"))
    (:NewEnumerator8
      (Audio|Components|Audio|SetSound _audiocomponent "/Game/Audio/BGM/SC_BGM_Market.SC_BGM_Market"))))