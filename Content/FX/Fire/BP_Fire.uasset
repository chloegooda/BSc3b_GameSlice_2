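; BP_Fire is a fire actor with standard, healing and poison types, where the healing type restores the player to full health.
; BeginPlay plays a spatialized crackle sound and selects the particle template from FireType.
; Box overlap calls HealPlayer if the player's CanBeHealedByFire flag is set.
; For healing fire only, HealPlayer applies the missing health to the player's UI and GI_Main game instance, then plays a pickup sound.
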(event OnComponentBeginOverlap(Box)
  (params (OverlappedComponent :type Primitive%20Component%20Object%20Reference) (OtherActor :type Actor%20Object%20Reference) (OtherComp :type Primitive%20Component%20Object%20Reference) (OtherBodyIndex :type Integer) (bFromSweep :type Boolean) (SweepResult :type Hit%20Result%20Structure%20%28by%20ref%29))
  (bind _asplayer_character (Utilities|Casting|CastToPlayerCharacter OtherActor))
  (if (Variables|/Game/ThirdPersonCharacter/PlayerCharacter.PlayerCharacter_C|GetCanBeHealedByFire? _asplayer_character)
    (CallFunction|HealPlayer)))

(event Custom|HealPlayer
  (if (== (Variables|Default|GetFireType) (Utilities|Enum|LiteralenumTypesOfFire "NewEnumerator1"))
    (bind _asgi_main (Utilities|Casting|CastToGI_Main (Game|GetGameInstance)))
    (bind _asplayer_character (Utilities|Casting|CastToPlayerCharacter (Game|GetPlayerCharacter 0)))
    (Default|ModifyHealthUI _asplayer_character (- (Variables|/Script/GameSlice.GI_Main|GetmaxPlayerHealth _asgi_main) (Variables|/Script/GameSlice.GI_Main|GetcurrentPlayerHealth _asgi_main)))
    (Class|GIMain|ModifyHealth _asgi_main (- (Variables|/Script/GameSlice.GI_Main|GetmaxPlayerHealth _asgi_main) (Variables|/Script/GameSlice.GI_Main|GetcurrentPlayerHealth _asgi_main)))
    (Audio|PlaySound2D "/Game/Audio/SFX/S_ItemPickup.S_ItemPickup" 1.0 1.0 0.0 0 0)))

(event EventBeginPlay
  (bind _fireparticlesystem (Variables|Default|GetFireParticleSystem))
  (Audio|PlaySoundatLocation "/Game/Audio/SFX/SC_FireCrackle.SC_FireCrackle" (Transformation|GetActorLocation) "0, 0, 0" 1.0 1.0 0.0 "/Game/Audio/SFX/SA_FireCrackle.SA_FireCrackle" 0 0)
  (switch Utilities|FlowControl|Switch|SwitchonTypesOfFire (Variables|Default|GetFireType)
    (:NewEnumerator0
      (Effects|Components|ParticleSystem|SetTemplate _fireparticlesystem "/Game/FX/Fire/P_FireEffect.P_FireEffect"))
    (:NewEnumerator1
      (Effects|Components|ParticleSystem|SetTemplate _fireparticlesystem "/Game/FX/Fire/P_HealingFireEffect.P_HealingFireEffect"))
    (:NewEnumerator2
      (Effects|Components|ParticleSystem|SetTemplate _fireparticlesystem "/Game/FX/Fire/P_EvilFireEffect.P_EvilFireEffect"))))

(fn ConstructionScript)