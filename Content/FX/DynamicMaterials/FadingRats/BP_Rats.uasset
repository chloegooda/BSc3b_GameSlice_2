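; BP_Rats is a rat actor that fades out and destroys itself when picked up.
; BeginPlay chooses a black or brown dynamic-ready material by comparing StaticMesh against the RatPack rat variants.
; PickUpRat creates a dynamic instance of that material, stored as BlackRat for either colour, and applies it to the mesh.
; A timeline drives the instance's Opacity parameter, then destroys the actor when finished.
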(event Custom|Pick%20Up%20Rat
  (Rendering|Material|SetMaterial (Variables|Default|GetStaticMesh) 0 (Variables|Default|GetMaterial))
  (bind _returnvalue (Rendering|Material|CreateDynamicMaterialInstance (Variables|Default|GetMaterial) "Dynamic_MI_RatsBlack" :!class /Script/Engine.KismetMaterialLibrary))
  (bind _output_get (Variables|Default|SetBlack%20Rat _returnvalue))
  (Rendering|Material|SetMaterial (Variables|Default|GetStaticMesh) 0 _output_get)
  (bind _percentage (Timeline|Timeline_0 Play)
    (:Update
      (Rendering|Material|SetScalarParameterValue (Variables|Default|GetBlack%20Rat) "Opacity" _percentage :!class /Script/Engine.MaterialInstanceDynamic))
    (:Finished
      (Actor|DestroyActor))))

(event EventBeginPlay
  (bind _staticmesh (Variables|Default|GetStaticMesh))
  (if (== _staticmesh "/Game/Assets/SM_Assets/Rats/RatPack_Rat2.RatPack_Rat2")
    (Variables|Default|SetMaterial "/Game/FX/DynamicMaterials/FadingRats/M_Rats_Dynamic_Black.M_Rats_Dynamic_Black")
    (elif (== _staticmesh "/Game/Assets/SM_Assets/Rats/RatPack_Rat3.RatPack_Rat3")
      (Variables|Default|SetMaterial "/Game/FX/DynamicMaterials/FadingRats/M_Rats_Dynamic_Brown.M_Rats_Dynamic_Brown"))))

(event Collision|EventActorBeginOverlap
  (params (OtherActor :type Actor%20Object%20Reference)))

(event EventTick
  (params (DeltaSeconds :type Float%20%28single-precision%29)))

(fn ConstructionScript)