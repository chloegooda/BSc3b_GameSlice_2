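; BP_RandomMapAsset_Ruin is a placement actor that spawns a random map asset at its location, apparently for ruins in enemy levels.
; On BeginPlay, AttemptToSpawn checks CurrentItem and either prints that an item already exists or calls SpawnItem.
; SpawnItem picks a random class from ItemsToSpawn, spawns it with random yaw, adjusting for collisions but always spawning, and stores it in CurrentItem.
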(event EventBeginPlay
  (CallFunction|AttempttoSpawn))

(fn ConstructionScript)

(fn SpawnItem
  (bind _itemstospawn (Variables|Default|GetItemsToSpawn))
  (bind _returnvalue (Game|SpawnActorfromClass (Utilities|Array|Get(acopy) _itemstospawn (Math|Random|RandomIntegerinRange 0 (- (Utilities|Array|Length _itemstospawn) 1))) (Math|Transform|MakeTransform (Transformation|GetActorLocation) (Math|Rotator|MakeRotator 0.0 0.0 (Math|Random|RandomFloatinRange 0.0 3.6e+02))) "AdjustIfPossibleButAlwaysSpawn" 0 0))
  (Variables|Default|SetCurrent%20Item _returnvalue))

(fn AttempttoSpawn
  (Utilities|IsValid (Variables|Default|GetCurrent%20Item)
    (:Is%20Valid
      (Development|PrintString "Item Already Spawned" true true "(R=1.000000,G=0.102968,B=0.000000,A=1.000000)"))
    (:Is%20Not%20Valid
      (CallFunction|SpawnItem))))