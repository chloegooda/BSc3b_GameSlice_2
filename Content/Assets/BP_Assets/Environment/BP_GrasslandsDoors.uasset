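; Grasslands double-door Blueprint that swings a pair of gates open and closed.
; OpenGates plays a timeline that yaws PivotL and PivotR in opposite directions, scaled to 90 degrees, and CloseGates reverses it from the end.
; An older fade and open-level-by-name path remains unconnected, noted as superseded by level streaming.
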(event Custom|OpenGates
  (bind _timeline (Timeline|Timeline_1 PlayFromStart)
    (:Update
      (Transformation|SetRelativeRotation (Variables|Default|GetPivotL) (Math|Rotator|MakeRotator 0.0 0.0 (* _timeline -9e+01)) false false)
      (Transformation|SetRelativeRotation (Variables|Default|GetPivotR) (Math|Rotator|MakeRotator 0.0 0.0 (* _timeline 9e+01)) false false))))

(event Custom|CloseGates
  (bind _timeline (Timeline|Timeline_1 ReverseFromEnd)
    (:Update
      (Transformation|SetRelativeRotation (Variables|Default|GetPivotL) (Math|Rotator|MakeRotator 0.0 0.0 (* _timeline -9e+01)) false false)
      (Transformation|SetRelativeRotation (Variables|Default|GetPivotR) (Math|Rotator|MakeRotator 0.0 0.0 (* _timeline 9e+01)) false false))))

(fn ConstructionScript
  (|CallParentFunction))