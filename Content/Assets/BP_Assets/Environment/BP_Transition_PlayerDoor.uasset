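; Player door that swings open on toggle and moves the player between scenes using level streaming.
; Toggle plays the open sound and rotation timeline while a scene transition runs with player movement suspended.
; After a delay it loads or unloads the linked level based on the entrance flag, teleports the player to the target location and updates the music.
; An older open-level method remains as disconnected nodes.
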(event Custom|LoadInLevel
  (bind _linkedlocation (Variables|Default|GetLinkedLocation))
  (bind _returnvalue (Utilities|String|EnumtoString _linkedlocation))
  (bind _returnvalue_2 (Utilities|String|StringToName _returnvalue))
  (Utilities|FlowControl|Delay 0.1)
  (Audio|PlaySound2D "/Game/Audio/SFX/S_DoorClose.S_DoorClose" 0.8 1.0 0.0 0 0)
  (if (Variables|Default|GetEntranceToLevel?)
    (Game|LoadStreamLevel(byName) _returnvalue_2 true)
    (bind _asbp_npc_quest_giver (Utilities|Casting|CastToBP_NPC_QuestGiver (Game|GetPlayerCharacter 0)))
    (Pawn|Components|CharacterMovement|SetMovementMode (Variables|/Script/Engine.Character|GetCharacterMovement _asbp_npc_quest_giver) "MOVE_Walking" 0)
    (else
      (bind _asbp_npc_quest_giver_2 (Utilities|Casting|CastToBP_NPC_QuestGiver (Game|GetPlayerCharacter 0))
        (:then
          (Pawn|Components|CharacterMovement|DisableMovement (Variables|/Script/Engine.Character|GetCharacterMovement _asbp_npc_quest_giver_2)))
        (:CastFailed
          _))
      (Game|UnloadStreamLevel(byName) _returnvalue_2 false))))

(event Custom|TransitionBetweenScenes
  (bind _returnvalue (Game|GetPlayerCharacter 0))
  (bind _charactermovement (Variables|/Script/Engine.Character|GetCharacterMovement _returnvalue))
  (Components|Activation|SetActive _charactermovement false false)
  (CallFunction|PlaySceneTransition false)
  (Utilities|FlowControl|Delay 1.0)
  (CallFunction|LoadinLevel)
  (Transformation|SetActorLocation _returnvalue (Transformation|GetActorLocation (Variables|Default|GetTeleportLocation)) false false)
  (Components|Activation|SetActive _charactermovement true false)
  (CallFunction|UpdateBGM))

(event EventToggle
  (CallFunction|TransitionBetweenScenes)
  (Audio|PlaySound2D "/Game/Audio/SFX/S_DoorOpen.S_DoorOpen" 0.8 1.0 0.0 0 0)
  (bind _timeline (Timeline|Timeline_1 Play)
    (:Update
      (Transformation|SetRelativeRotation (Variables|Default|GetPivot) (Math|Rotator|MakeRotator 0.0 0.0 (* _timeline 9e+01)) false false))
    (:Finished
      (Transformation|SetRelativeRotation (Variables|Default|GetPivot) (Math|Rotator|MakeRotator 0.0 0.0 0.0) false false))))

(fn ConstructionScript
  (|CallParentFunction))