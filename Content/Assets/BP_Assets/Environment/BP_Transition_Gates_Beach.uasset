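; Beach transition gate Blueprint that moves between scenes when the player is allowed entry.
; Toggle passes the player character's CanEnterBeachGate flag to CanEnterGates, which does nothing if entry is denied.
; On success it calls TransitionBetweenScenes, plays the gate-open sound and runs a timeline that swings the two pivots outward in opposite yaw, snapping both back to closed when it finishes.
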(event Custom|Can%20Enter%20Gates?
  (params (Entry%20Allowed? :type Boolean))
  (if Entry%20Allowed?
    (CallFunction|TransitionBetweenScenes)
    (Audio|PlaySound2D "/Game/Audio/SFX/S_GateOpen.S_GateOpen" 0.7 1.0 0.0 0 0)
    (bind _timeline (Timeline|Timeline_2 PlayFromStart)
      (:Update
        (Transformation|SetRelativeRotation (Variables|Default|GetPivotL) (Math|Rotator|MakeRotator 0.0 0.0 (* _timeline -9e+01)) false false)
        (Transformation|SetRelativeRotation (Variables|Default|GetPivotR) (Math|Rotator|MakeRotator 0.0 0.0 (* _timeline 9e+01)) false false))
      (:Finished
        (Transformation|SetRelativeRotation (Variables|Default|GetPivotL) (Math|Rotator|MakeRotator 0.0 0.0 0.0) false false)
        (Transformation|SetRelativeRotation (Variables|Default|GetPivotR) (Math|Rotator|MakeRotator 0.0 0.0 0.0) false false)))))

(event EventBeginPlay)

(event Collision|EventActorBeginOverlap
  (params (OtherActor :type Actor%20Object%20Reference)))

(event EventTick
  (params (DeltaSeconds :type Float%20%28single-precision%29)))

(event EventToggle
  (bind _asplayer_character (Utilities|Casting|CastToPlayerCharacter (Game|GetPlayerCharacter 0)))
  (CallFunction|CanEnterGates? (Variables|/Game/ThirdPersonCharacter/PlayerCharacter.PlayerCharacter_C|GetCanEnterBeachGate? _asplayer_character)))

(fn ConstructionScript
  (|CallParentFunction))