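; Interactable rat actor for Chloe and Becky, which the player can talk to and which fades out before being picked up.
; BeginPlay picks a black or brown dynamic-ready material according to the rat's mesh.
; TalkToRat opens that rat's interaction widget by Name, switches to UI-only input with a cursor and halts player movement.
; FadeoutRat creates a dynamic material instance, drives its Opacity with a timeline, then calls PickUpItem.
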(event Custom|Talk%20To%20Rat
  (bind _returnvalue (Game|GetPlayerController 0))
  (bind _returnvalue_2 (Game|GetPlayerController 0))
  (if (Utilities|Enum|Equal(Enum) (Variables|Default|GetName) (Variables|Default|GetBecky))
    (bind _returnvalue_3 (UserInterface|CreateWidget "/Game/UI/Rats/BPW_BeckyInteract.BPW_BeckyInteract_C"))
    (UserInterface|Viewport|AddtoViewport _returnvalue_3 0)
    (Input|SetInputModeUIOnly _returnvalue _returnvalue_3 "DoNotLock")
    (Variables|/Script/Engine.PlayerController|SetbShowMouseCursor _returnvalue true)
    (bind _asplayer_character (Utilities|Casting|CastToPlayerCharacter (Game|GetPlayerCharacter 0) :!label _label))
    (Pawn|Components|CharacterMovement|SetMovementMode (Variables|/Script/Engine.Character|GetCharacterMovement _asplayer_character) "MOVE_None" 0)
    (elif (Utilities|Enum|Equal(Enum) (Variables|Default|GetName) (Variables|Default|GetChloe))
      (bind _returnvalue_4 (UserInterface|CreateWidget "/Game/UI/Rats/BPW_ChloeInteract.BPW_ChloeInteract_C"))
      (UserInterface|Viewport|AddtoViewport _returnvalue_4 0)
      (Input|SetInputModeUIOnly _returnvalue_2 _returnvalue_4 "DoNotLock")
      (Variables|/Script/Engine.PlayerController|SetbShowMouseCursor _returnvalue_2 true)
      (goto _label))))

(event Custom|Fade%20out%20Rat
  (Rendering|Material|SetMaterial (Variables|Default|GetMeshComponent) 0 (Variables|Default|GetMaterial))
  (bind _returnvalue (Rendering|Material|CreateDynamicMaterialInstance (Variables|Default|GetMaterial) "Dynamic_MI_RatsBlack" :!class /Script/Engine.KismetMaterialLibrary))
  (bind _output_get (Variables|Default|SetBlack%20Rat _returnvalue))
  (Rendering|Material|SetMaterial (Variables|Default|GetMeshComponent) 0 _output_get)
  (bind _percentage (Timeline|Timeline_0 Play)
    (:Update
      (Rendering|Material|SetScalarParameterValue (Variables|Default|GetBlack%20Rat) "Opacity" _percentage :!class /Script/Engine.MaterialInstanceDynamic))
    (:Finished
      (Class|KeyItem|PickUpItem))))

(event EventBeginPlay
  (if (== 0 "/Game/Assets/SM_Assets/Rats/SM_Rat_Chloe.SM_Rat_Chloe")
    (Variables|Default|SetMaterial "/Game/FX/DynamicMaterials/FadingRats/M_Rats_Dynamic_Black.M_Rats_Dynamic_Black")
    (elif (== 0 "/Game/Assets/SM_Assets/Rats/SM_Rat_Becky.SM_Rat_Becky")
      (Variables|Default|SetMaterial "/Game/FX/DynamicMaterials/FadingRats/M_Rats_Dynamic_Brown.M_Rats_Dynamic_Brown"))))

(event Collision|EventActorBeginOverlap
  (params (OtherActor :type Actor%20Object%20Reference)))

(event EventTick
  (params (DeltaSeconds :type Float%20%28single-precision%29)))

(fn ConstructionScript)