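; Transition gate that moves the player and companion AI out of the enemy level, using level streaming.
; Toggle grants beach-gate access if tagged BeachGate, then starts the transition and swings both gate pivots on a timeline, resetting them afterwards.
; The transition pauses player movement, plays a screen transition, loads or unloads LinkedLocation based on EntranceToLevel, teleports player and first AI_NewCharacter, updates music and unloads LV_EnemyArea.
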(event Custom|LoadInLevel
  (bind _linkedlocation (Variables|Default|GetLinkedLocation))
  (bind _returnvalue (Utilities|String|EnumtoString _linkedlocation))
  (bind _returnvalue_2 (Utilities|String|StringToName _returnvalue))
  (Utilities|FlowControl|Delay 0.1)
  (Audio|PlaySound2D "/Game/Audio/SFX/S_GateClose.S_GateClose" 0.7 1.0 0.0 0 0)
  (if (Variables|Default|GetEntranceToLevel?)
    (Game|LoadStreamLevel(byName) _returnvalue_2 true)
    (bind _asbp_npc_quest_giver (Utilities|Casting|CastToBP_NPC_QuestGiver (Game|GetPlayerCharacter 0)))
    (Pawn|Components|CharacterMovement|SetMovementMode (Variables|/Script/Engine.Character|GetCharacterMovement _asbp_npc_quest_giver) "MOVE_Walking" 0)
    (else
      (bind _asbp_npc_quest_giver_2 (Utilities|Casting|CastToBP_NPC_QuestGiver (Game|GetPlayerCharacter 0))
        (:then
          (Pawn|Components|CharacterMovement|DisableMovement (Variables|/Script/Engine.Character|GetCharacterMovement _asbp_npc_quest_giver_2)))
        (:CastFailed
          _))
      (Game|UnloadStreamLevel(byName) _returnvalue_2 false))))

(event Custom|TransitionBetweenScenes
  (bind _returnvalue (Game|GetPlayerCharacter 0))
  (bind _charactermovement (Variables|/Script/Engine.Character|GetCharacterMovement _returnvalue))
  (Components|Activation|SetActive _charactermovement false false)
  (CallFunction|PlaySceneTransition false)
  (Utilities|FlowControl|Delay 1.0)
  (CallFunction|LoadinLevel)
  (Transformation|SetActorLocation _returnvalue (Transformation|GetActorLocation (Variables|Default|GetTeleportLocation)) false false)
  (Utilities|FlowControl|Delay 1.0)
  (Components|Activation|SetActive _charactermovement true false)
  (bind _outactors (Actor|GetAllActorsOfClass "/Game/AI/NewAI/AI_NewCharacter.AI_NewCharacter_C"))
  (Transformation|SetActorLocation (Utilities|Array|Get(acopy) _outactors) (Transformation|GetActorLocation (Variables|Default|GetAITeleportLocation)) false false)
  (CallFunction|UpdateBGM)
  (Game|UnloadStreamLevel(byName) "LV_EnemyArea" false))

(event EventToggle
  (if (Actor|ActorHasTag "BeachGate")
    (bind _asplayer_character (Utilities|Casting|CastToPlayerCharacter (Game|GetPlayerCharacter 0)))
    (Variables|/Game/ThirdPersonCharacter/PlayerCharacter.PlayerCharacter_C|SetCanEnterBeachGate? _asplayer_character true))
  (CallFunction|TransitionBetweenScenes)
  (Audio|PlaySound2D "/Game/Audio/SFX/S_GateOpen.S_GateOpen" 0.7 1.0 0.0 0 0)
  (bind _timeline (Timeline|Timeline_1 PlayFromStart)
    (:Update
      (Transformation|SetRelativeRotation (Variables|Default|GetPivotL) (Math|Rotator|MakeRotator 0.0 0.0 (* _timeline -9e+01)) false false)
      (Transformation|SetRelativeRotation (Variables|Default|GetPivotR) (Math|Rotator|MakeRotator 0.0 0.0 (* _timeline 9e+01)) false false))
    (:Finished
      (Transformation|SetRelativeRotation (Variables|Default|GetPivotL) (Math|Rotator|MakeRotator 0.0 0.0 0.0) false false)
      (Transformation|SetRelativeRotation (Variables|Default|GetPivotR) (Math|Rotator|MakeRotator 0.0 0.0 0.0) false false))))

(fn ConstructionScript
  (|CallParentFunction))