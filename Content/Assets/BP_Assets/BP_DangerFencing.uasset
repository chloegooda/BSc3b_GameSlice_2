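; BP_DangerFencing is a fence actor that removes itself once the player has the "training_dummies" skill point.
; Any overlap on its Box triggers CheckFencing, which queries player 0's BPSkillPointsComponent and destroys the actor if the point is present.
; Leftover test nodes for a looping timer and a delayed grant of that point are disconnected and never run.
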(event OnComponentBeginOverlap(Box)
  (params (OverlappedComponent :type Primitive%20Component%20Object%20Reference) (OtherActor :type Actor%20Object%20Reference) (OtherComp :type Primitive%20Component%20Object%20Reference) (OtherBodyIndex :type Integer) (bFromSweep :type Boolean) (SweepResult :type Hit%20Result%20Structure%20%28by%20ref%29))
  (CallFunction|CheckFencing))

(event Custom|CheckFencing
  (bind _asplayer_character (Utilities|Casting|CastToPlayerCharacter (Game|GetPlayerCharacter 0)))
  (bind _success (Default|QueryPoint (Variables|/Game/ThirdPersonCharacter/PlayerCharacter.PlayerCharacter_C|GetBP_SkillPointsComponent _asplayer_character) "training_dummies"))
  (if _success
    (Actor|DestroyActor)))

(event EventBeginPlay)

(fn ConstructionScript)