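; Combat director that picks which enemy in EnemyList attacks, on a looping timer.
; Each tick scales every enemy's grade by how opposed its forward vector is to the player's, favoring face-to-face enemies.
; The top-graded enemy's AIC_Enemies controller runs AIAttack, then that enemy gets a new random grade.
; Grades live in the EnemyGrading map and show on debug widgets attached to each enemy at BeginPlay.
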(event Custom|Trigger%20Attack
  (CallFunction|RecalculateScores)
  (bind _highestgradedai1 (CallFunction|FindHighestGrading))
  (bind _asaic_enemies (Utilities|Casting|CastToAIC_Enemies (AI|GetAIController _highestgradedai1)))
  (Default|AIAttack _asaic_enemies)
  (Utilities|Map|Add (Variables|Default|GetEnemyGrading) _highestgradedai1 (Math|Random|RandomFloatinRange 1.0 5.0))
  (CallFunction|UpdateDebugWidgets _highestgradedai1))

(event EventBeginPlay
  (for _array_element (Variables|Default|GetEnemyList)
    (CallFunction|AddDebugWidgets _array_element))
  (Utilities|Time|SetTimerbyEvent (delegate Custom|Trigger%20Attack) 4.0 true))

(fn ConstructionScript)

(fn FindHighestGrading
  (bind _keys (Utilities|Map|Keys (Variables|Default|GetEnemyGrading)))
  (for _array_element _keys
    (if (> (.Value (Utilities|Map|Find (Variables|Default|GetEnemyGrading) _array_element)) (LocalVariables|GetHighestValue))
      (LocalVariables|SetHighestValue (.Value (Utilities|Map|Find (Variables|Default|GetEnemyGrading) _array_element)))
      (LocalVariables|SetHighestGradedAI _array_element)))
  (return (LocalVariables|GetHighestValue) (LocalVariables|GetHighestGradedAI)))

(fn AddDebugWidgets
  (params (Enemy%20Instance :type BP%20Enemy%20Basic%20Object%20Reference%20%28by%20ref%29))
  (Utilities|Map|Add (Variables|Default|GetEnemyGrading) Enemy%20Instance (Math|Random|RandomFloatinRange 1.0 5.0))
  (bind _returnvalue (UserInterface|CreateWidget "/Game/Enemies/BPW_DebugEnemyCombat.BPW_DebugEnemyCombat_C" 0 Enemy%20Instance (.Value (Utilities|Map|Find (Variables|Default|GetEnemyGrading) Enemy%20Instance))))
  (bind _output_get (LocalVariables|SetWidget _returnvalue))
  (Utilities|Map|Add (Variables|Default|GetEnemy%20Widgets) Enemy%20Instance _output_get)
  (bind _returnvalue_2 (AddComponent|AddWidgetComponent Enemy%20Instance false))
  (UserInterface|SetWidget _returnvalue_2 (LocalVariables|GetWidget)))

(fn UpdateDebugWidgets
  (params (Enemy%20Instance :type BP%20Enemy%20Basic%20Object%20Reference))
  (Variables|/Game/Enemies/BPW_DebugEnemyCombat.BPW_DebugEnemyCombat_C|SetFighting%20Grade (.Value (Utilities|Map|Find (Variables|Default|GetEnemy%20Widgets) Enemy%20Instance)) (.Value (Utilities|Map|Find (Variables|Default|GetEnemyGrading) Enemy%20Instance))))

(fn RecalculateScores
  (CallFunction|ScorebyPosition))

(fn ScorebyPosition
  (bind _enemygrading (Variables|Default|GetEnemyGrading))
  (for _array_element (Variables|Default|GetEnemyList)
    (Development|PrintString (Utilities|String|ToString(Float) (* (Math|Vector|DotProduct (Transformation|GetActorForwardVector _array_element) (Transformation|GetActorForwardVector (Game|GetPlayerCharacter 0))) -1.0)))
    (Utilities|Map|Add _enemygrading _array_element (* (.Value (Utilities|Map|Find _enemygrading _array_element)) (+ (Math|Float|NormalizetoRange (* (Math|Vector|DotProduct (Transformation|GetActorForwardVector _array_element) (Transformation|GetActorForwardVector (Game|GetPlayerCharacter 0))) -1.0) -1.0 1.0) 0.5)))
    (CallFunction|UpdateDebugWidgets _array_element)))