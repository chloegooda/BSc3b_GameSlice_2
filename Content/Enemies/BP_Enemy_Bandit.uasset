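; Bandit enemy Blueprint with a health bar widget, simple damage handling and quest kill reporting.
; On BeginPlay it links itself to the health bar widget and starts a looping one-second timer that checks for death.
; Once dead, it destroys itself a single time, then notifies every quest in the player's quest log of the kill.
; TakeDamage removes one clamped health point per call and updates the health percentage.
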(event Custom|Check%20Enemy%20Health
  (Class|EnemyBase|EnemyHasNoHealth false)
  (if (Variables|Default|GetEnemyDead)
    (Utilities|FlowControl|DoOnce false
      (:Completed
        (Actor|DestroyActor)
        (bind _asplayer_character (Utilities|Casting|CastToPlayerCharacter (Game|GetPlayerCharacter 0)))
        (for _array_element (Variables|/Game/QuestSystem/Blueprints/BP_QuestLog.BP_QuestLog_C|GetQuests (Variables|/Game/ThirdPersonCharacter/PlayerCharacter.PlayerCharacter_C|GetBP_QuestLog _asplayer_character))
          (Default|CallKilledEnemy _array_element self))))))

(event EventBeginPlay
  (bind _asbpw_new_health_bar (Utilities|Casting|CastToBPW_NewHealthBar (UserInterface|GetUserWidgetObject (Variables|Default|GetEnemyHealthBar))))
  (Variables|/Game/UI/HealthSystem/BPW_NewHealthBar.BPW_NewHealthBar_C|SetEnemy _asbpw_new_health_bar self)
  (Utilities|Time|SetTimerbyEvent (delegate Custom|Check%20Enemy%20Health) 1.0 true))

(fn ConstructionScript)

(fn TakeDamage
  (bind _output_get (Variables|Default|SetCurrentHealth (Math|Float|Clamp(Float) (- (Variables|Default|GetCurrentHealth) 1.0) 0.0 5.0)))
  (Variables|Default|SetHealthPercentage (/ _output_get (Variables|Default|GetMaxHealth))))