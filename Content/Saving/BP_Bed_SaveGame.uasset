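; Bed save point Blueprint that saves player progress through an OverwriteSaveGame event.
; The event creates a fresh SaveGameFile object and fills PlayerSaveInfo with gold, health, unlocked weapon classes and item lists from GI_Main, plus skill points from PlayerCharacter.
; It writes to the save object's own slot name and user index, replacing prior data, then prints a saving message.
; Nothing in this Blueprint calls the event.
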(event EventBeginPlay)

(event Collision|EventActorBeginOverlap
  (params (OtherActor :type Actor%20Object%20Reference)))

(event EventTick
  (params (DeltaSeconds :type Float%20%28single-precision%29)))

(event EventOverwriteSaveGame
  (bind _returnvalue (SaveGame|CreateSaveGameObject "/Script/GameSlice.SaveGameFile"))
  (bind _output_get (Variables|Default|SetSaveGameInstance _returnvalue))
  (bind _asgi_main (Utilities|Casting|CastToGI_Main (Game|GetGameInstance)))
  (bind _asplayer_character (Utilities|Casting|CastToPlayerCharacter (Game|GetPlayerCharacter 0)))
  (Variables|/Script/GameSlice.SaveGameFile|SetPlayerSaveInfo _output_get (Utilities|Struct|MakePlayerSaveInfo (Variables|/Script/GameSlice.GI_Main|GetplayerGold _asgi_main) (Variables|/Game/ThirdPersonCharacter/PlayerCharacter.PlayerCharacter_C|GetSkillPoints _asplayer_character) (Variables|/Script/GameSlice.GI_Main|GetcurrentPlayerHealth _asgi_main) (Variables|/Script/GameSlice.GI_Main|GetUnlockedWeaponClasses _asgi_main) (Variables|/Script/GameSlice.GI_Main|GetItemList _asgi_main) (Variables|/Script/GameSlice.GI_Main|GetKeyItemList _asgi_main)))
  (SaveGame|SaveGametoSlot _output_get (Variables|/Script/GameSlice.SaveGameFile|GetSaveSlotName _output_get) (Variables|/Script/GameSlice.SaveGameFile|GetUserIndex _output_get))
  (Development|PrintString "SAVING..."))

(fn ConstructionScript)