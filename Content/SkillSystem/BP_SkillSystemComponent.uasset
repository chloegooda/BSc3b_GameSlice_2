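; Skill system component that tracks which skills its owner has unlocked and at what tier, in a SkillUnlocks map keyed by row name.
; Add Skill inserts a new skill at tier one or increments an existing one, with no cap or validation, and returns false on both paths.
; Query Skill reports whether a row name is unlocked and its tier level, or zero when absent.
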(event EventBeginPlay)

(event EventTick
  (params (DeltaSeconds :type Float%20%28single-precision%29)))

(fn AddSkill
  (params (row_name :type String))
  (bind _skill_unlocks (Variables|Default|GetSkill%20Unlocks))
  (bind (_value _returnvalue) (Utilities|Map|Find _skill_unlocks row_name))
  (if _returnvalue
    (Utilities|Map|Add (Variables|Default|GetSkill%20Unlocks) row_name (+ _value 1))
    (return false)
    (else
      (Utilities|Map|Add (Variables|Default|GetSkill%20Unlocks) row_name 1)
      (return false))))

(fn QuerySkill
  (params (row_name :type String))
  (bind _skill_unlocks (Variables|Default|GetSkill%20Unlocks))
  (bind (_value _returnvalue) (Utilities|Map|Find _skill_unlocks row_name))
  (if _returnvalue
    (return true _value)
    (else
      (return false 0))))