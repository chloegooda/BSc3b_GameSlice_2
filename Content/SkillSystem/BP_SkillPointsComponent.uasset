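; BP_SkillPointsComponent is a skill system component that records points spent on skills in a PointsUnlocks map keyed by row name.
; AddPoint increments the stored count or inserts a new entry at 1, and returns false on both paths.
; QueryPoint reports only whether a row has an entry, without exposing its point count.
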(event EventBeginPlay)

(event EventTick
  (params (DeltaSeconds :type Float%20%28single-precision%29)))

(fn AddPoint
  (params (row_name :type String))
  (bind _points_unlocks (Variables|Default|GetPoints%20Unlocks))
  (bind (_value _returnvalue) (Utilities|Map|Find _points_unlocks row_name))
  (if _returnvalue
    (Utilities|Map|Add (Variables|Default|GetPoints%20Unlocks) row_name (+ _value 1))
    (return false)
    (else
      (Utilities|Map|Add (Variables|Default|GetPoints%20Unlocks) row_name 1)
      (return false))))

(fn QueryPoint
  (params (row_name :type String))
  (if (.ReturnValue (Utilities|Map|Find (Variables|Default|GetPoints%20Unlocks) row_name))
    (return true)
    (else
      (return false))))